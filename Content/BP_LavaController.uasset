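; BP_LavaController is a controller Blueprint that toggles a debug widget and the mouse cursor with the H key.
; The first press creates the widget and adds it to the viewport, and later presses switch it between visible and collapsed.
; Each press also ensures a post process component exists on player character 0, adding one and caching it as PP if missing.
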(event Input|KeyboardEvents|H
  (params (Key :type Key%20Structure :default "None"))
  (:Pressed
    (Utilities|IsValid (Variables|Default|GetPP)
      (:Is%20Valid
        _)
      (:Is%20Not%20Valid
        (bind _returnvalue (AddComponent|AddPostProcessComponent (Game|GetPlayerCharacter 0) false))
        (Variables|Default|SetPP _returnvalue)))
    (Utilities|IsValid (Variables|Default|GetDebug)
      (:Is%20Valid
        (if (Widget|IsVisible (Variables|Default|GetDebug))
          (Widget|SetVisibility (Variables|Default|GetDebug) "Collapsed")
          (Variables|Default|SetbShowMouseCursor false)
          (else
            (Widget|SetVisibility (Variables|Default|GetDebug) "Visible")
            (Variables|Default|SetbShowMouseCursor true))))
      (:Is%20Not%20Valid
        (bind _returnvalue_2 (UserInterface|CreateWidget "/Game/Debug/DebugWidget.DebugWidget_C"))
        (UserInterface|Viewport|AddtoViewport _returnvalue_2 0)
        (Variables|Default|SetDebug _returnvalue_2)
        (Variables|Default|SetbShowMouseCursor true)))))

(fn ConstructionScript)